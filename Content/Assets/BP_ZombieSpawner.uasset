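; Zombie spawner actor that runs wave-based rounds for a zombie soccer game, spawning enemies at its own location.
; A looping timer, with its interval randomized once at BeginPlay, spawns either a regular or sprinter zombie while the round's count lasts, favoring regulars.
; When the count runs out, it advances the round, sets the next count from the round number, increments the GM_ZombieSoccer round and plays a cue.
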(event Custom|SpawnZombies
  (if (> (Variables|Default|GetNumberOfZombiesToSpawn) 0)
    (bind _output_get (Variables|Default|SetNumberOfZombiesToSpawn (Variables|Default|GetNumberOfZombiesToSpawn)))
    (bind _result (Math|Integer|DecrementInt _output_get)
      (:%20%20
        (Development|PrintString (Utilities|String|BuildString(Integer) "" "" _result " more Zombies will spawn this round!"))
        (if (> (Math|Random|RandomFloatinRange 1.0 3.0) 1.5)
          (CallFunction|SpawnZombie)
          (Development|PrintString ">> A Zombie has spawned!" true true "(R=1.000000,G=0.235294,B=0.196078,A=1.000000)")
          (else
            (CallFunction|SpawnZombieSprinter)
            (Development|PrintString ">> A Sprinter Zombie has spawned!" true true "(R=1.000000,G=0.235294,B=0.196078,A=1.000000)")))))
    (else
      (bind _output_get_2 (Variables|Default|SetRoundNumber (Variables|Default|GetRoundNumber)))
      (bind _result_2 (Math|Integer|IncrementInt _output_get_2)
        (:%20%20
          (Development|PrintString (Utilities|String|BuildString(Integer) "Round #" "" _result_2 "!"))
          (bind _output_get_3 (Variables|Default|SetNumberOfZombiesToSpawn (* (Variables|Default|GetRoundNumber) 3)))
          (Development|PrintString (Utilities|String|BuildString(Integer) "" "" _output_get_3 " Zombies will be spawning this round!"))
          (bind _asgm_zombie_soccer (Utilities|Casting|CastToGM_ZombieSoccer (Game|GetGameMode)))
          (bind _output_get_4 (Variables|/Game/GM_ZombieSoccer.GM_ZombieSoccer_C|SetRound _asgm_zombie_soccer (Variables|/Game/GM_ZombieSoccer.GM_ZombieSoccer_C|GetRound _asgm_zombie_soccer)))
          (Math|Integer|IncrementInt _output_get_4
            (:%20%20
              (Audio|PlaySound2D "/Game/Sounds+Music/newRound_Cue.newRound_Cue" 1.0 1.0 0.0 0 0))))))))

(event EventBeginPlay
  (Utilities|Time|SetTimerbyEvent (delegate Custom|SpawnZombies) (Math|Random|RandomFloatinRange 5.0 1e+01) true))

(fn ConstructionScript)

(fn SpawnZombie
  (AI|SpawnAIFromClass "/Game/Assets/BP_Zombie.BP_Zombie_C" 0 (Transformation|GetActorLocation) (Transformation|GetActorRotation) false 0))

(fn SpawnZombieSprinter
  (AI|SpawnAIFromClass "/Game/Assets/BP_ZombieSprinter.BP_ZombieSprinter_C" 0 (Transformation|GetActorLocation) (Transformation|GetActorRotation) false 0))