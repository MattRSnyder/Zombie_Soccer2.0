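; Soccer ball actor that the player kicks with a weak (left click) or strong (right click) shot.
; Overlap with a BP_SoccerPlayer in the AllowPlayertoKick volume toggles the ball's input.
; Kicks apply a velocity-change impulse along the player pawn's forward vector, with sound, Niagara effect and debug text.
; Strong kicks briefly set LongShot after a delay; the BallDMG damage logic is unconnected and KickEnable is empty.
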(event OnComponentBeginOverlap(AllowPlayertoKick)
  (params (OverlappedComponent :type Primitive%20Component%20Object%20Reference) (OtherActor :type Actor%20Object%20Reference) (OtherComp :type Primitive%20Component%20Object%20Reference) (OtherBodyIndex :type Integer) (bFromSweep :type Boolean) (SweepResult :type Hit%20Result%20Structure%20%28by%20ref%29))
  ;[1 0.477 0.8622] Allow Player to Kick
  (Utilities|Casting|CastToBP_SoccerPlayer OtherActor)
  (Input|EnableInput (Game|GetPlayerController 0)))

(event OnComponentEndOverlap(AllowPlayertoKick)
  (params (OverlappedComponent :type Primitive%20Component%20Object%20Reference) (OtherActor :type Actor%20Object%20Reference) (OtherComp :type Primitive%20Component%20Object%20Reference) (OtherBodyIndex :type Integer))
  ;[1 0.477 0.8622] Allow Player to Kick
  (Utilities|Casting|CastToBP_SoccerPlayer OtherActor)
  (Input|DisableInput (Game|GetPlayerController 0)))

(event Input|MouseEvents|RightMouseButton
  (params (Key :type Key%20Structure :default "None"))
  ;[0.5059 1 0.5446] Strong Kick
  (:Pressed
    (Physics|AddImpulse (Variables|Debug|GetStaticMeshComponent) (* (Transformation|GetActorForwardVector (Game|Player|GetPlayerPawn 0)) (Variables|Default|GetStrongKick)) "None" true)
    (Development|PrintString "Strong Kick!" true true "(R=1.000000,G=0.882186,B=0.162187,A=1.000000)")
    (Audio|PlaySound2D "/Game/Sounds+Music/StrongKick_C.StrongKick_C" 1.0 1.0 0.0 0 0)
    (AddComponent|AddNiagaraComponent false)
    (Utilities|FlowControl|Delay 0.3)
    (Variables|Default|SetLongShot true)
    (Utilities|FlowControl|Delay 0.5)
    (Variables|Default|SetLongShot false)))

(event Input|MouseEvents|LeftMouseButton
  (params (Key :type Key%20Structure :default "None"))
  ;[0.5059 1 0.5446] Weak Kick
  (:Pressed
    (Physics|AddImpulse (Variables|Debug|GetStaticMeshComponent) (* (Transformation|GetActorForwardVector (Game|Player|GetPlayerPawn 0)) (Variables|Default|GetWeakKick)) "None" true)
    (Development|PrintString "Weak Kick!" true true "(R=1.000000,G=0.882186,B=0.162187,A=1.000000)")
    (Audio|PlaySound2D "/Game/Sounds+Music/weakKick_Cue.weakKick_Cue" 1.0 1.0 0.0 0 0)
    (AddComponent|AddNiagaraComponent false)))

(fn ConstructionScript)

(fn KickEnable)