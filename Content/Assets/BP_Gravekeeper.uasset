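; BP_Gravekeeper is an interactable actor that opens and closes the upgrades shop.
; An overlapping living soccer player triggers the intro of its Press E widget component, and leaving plays the outro, both with sound cues.
; The OpenShop event, not called within this file, toggles on a ShopOpen flag, swapping the HUD and shop widgets and switching input mode and mouse cursor.
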(event Custom|Open%20Shop
  (bind _returnvalue (Game|GetPlayerController 0))
  (if (Variables|Default|GetShopOpen)
    (Development|PrintString "Shop Closed!")
    (bind _foundwidgets (Widget|GetAllWidgetsOfClass "/Game/HUD/HUD_UpgradesShop.HUD_UpgradesShop_C" true))
    (Widget|RemovefromParent _foundwidgets)
    (Input|SetInputModeGameOnly _returnvalue)
    (Variables|/Script/Engine.PlayerController|SetbShowMouseCursor _returnvalue false)
    (bind _returnvalue_2 (UserInterface|CreateWidget "/Game/HUD/HUD_Widget.HUD_Widget_C" (Game|GetPlayerController 0)))
    (UserInterface|Viewport|AddtoViewport _returnvalue_2 0)
    (Audio|PlaySound2D "/Game/Sounds+Music/close_Cue.close_Cue" 1.0 1.0 0.0 0 0)
    (Variables|Default|SetShopOpen false)
    (else
      (Audio|PlaySound2D "/Game/Sounds+Music/open_Cue.open_Cue" 1.0 1.0 0.0 0 0)
      (bind _returnvalue_3 (UserInterface|CreateWidget "/Game/HUD/HUD_UpgradesShop.HUD_UpgradesShop_C" _returnvalue))
      (UserInterface|Viewport|AddtoViewport _returnvalue_3 0)
      (bind _foundwidgets_2 (Widget|GetAllWidgetsOfClass "/Game/HUD/HUD_Widget.HUD_Widget_C" true))
      (Widget|RemovefromParent _foundwidgets_2)
      (Input|SetInputModeGameandUI _returnvalue _returnvalue_3 "DoNotLock" true)
      (Variables|/Script/Engine.PlayerController|SetbShowMouseCursor _returnvalue true)
      (Variables|Default|SetShopOpen true)
      (Development|PrintString "Shop Opened!"))))

(event EventBeginPlay
  (bind _ashud_press_eoverlay (Utilities|Casting|CastToHUD_PressEOverlay (UserInterface|GetUserWidgetObject (Variables|Default|GetPressE))))
  (Variables|Default|SetW_PressE _ashud_press_eoverlay))

(event Collision|EventActorBeginOverlap
  (params (OtherActor :type Actor%20Object%20Reference))
  (bind _asbp_soccer_player (Utilities|Casting|CastToBP_SoccerPlayer OtherActor))
  (if (Variables|/Game/Assets/BP_SoccerPlayer.BP_SoccerPlayer_C|GetIsAlive _asbp_soccer_player)
    (Default|PlayIntro (Variables|Default|GetW_PressE))
    (Audio|PlaySound2D "/Game/Sounds+Music/pressEappears_Cue.pressEappears_Cue" 1.0 1.0 0.0 0 0)))

(event Collision|EventActorEndOverlap
  (params (OtherActor :type Actor%20Object%20Reference))
  (Utilities|Casting|CastToBP_SoccerPlayer OtherActor)
  (Default|PlayOutro (Variables|Default|GetW_PressE))
  (Audio|PlaySound2D "/Game/Sounds+Music/pressEdisappears_Cue.pressEdisappears_Cue" 1.0 1.0 0.0 0 0))

(fn ConstructionScript)